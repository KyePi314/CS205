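; Game instance Blueprint that prototypes saving and loading the player's position through a SaveGame_BP object.
; Save records the player location, or creates the save object if missing without recording it, then stamps the date and saves asynchronously to the Name slot.
; Load is unfinished: it only loops existence checks on an empty slot name.
; The load-or-create logic that would restore the player's position is disconnected and never runs.
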(event `Save`
  (`/Engine/EditorBlueprintResources/StandardMacros.IsValid` (`self.SaveGame`)
    (:`Is Valid`
      (set `/Game/SaveGame_BP.PlayerPos` (`Actor.K2_GetActorLocation` (`GameplayStatics.GetPlayerCharacter` 0)) (`self.SaveGame`)))
    (:`Is Not Valid`
      (bind _returnvalue (`GameplayStatics.CreateSaveGameObject` "/Game/SaveGame_BP.SaveGame_BP_C"))
      (bind _output_get (set `self.SaveGame` _returnvalue))
      (bind _output_get_2 (set `self.Name` ""))))
  (set `self.SaveDate` (`KismetMathLibrary.Now`))
  (`AsyncActionHandleSaveGame.AsyncSaveGameToSlot` _output_get (`KismetTextLibrary.Conv_TextToString` _output_get_2)
    (:`Completed`
      (`KismetSystemLibrary.PrintString` "Hello"))))

(event `Load`
  (for _index (range 11)
    (`GameplayStatics.DoesSaveGameExist` "")))