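; Player character Blueprint that handles camera-relative movement, jumping, sprinting, interaction and health.
; Interact sends InteractMessage to the last actor overlapping the capsule if it implements the FishingSpot_Bp interface.
; Damage lowers clamped health and refreshes a health bar widget created on BeginPlay; key 1 applies self-damage.
; P opens a pause menu and pauses the game; a GameInstance load call is left unconnected.
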(event `InputAction|InteractButton`
  (params (Key :type "Key Structure"))
  (bind _overlappingactors (`PrimitiveComponent.GetOverlappingActors` (`self.CapsuleComponent`) null))
  (bind _output (`|GetArrayItem` _overlappingactors (`KismetArrayLibrary.Array_LastIndex` _overlappingactors)))
  (:`Pressed`
    (if (`KismetSystemLibrary.DoesImplementInterface` _output "/Game/FishingSpot_Bp.FishingSpot_Bp_C")
      (message `/Game/FishingSpot_Bp.Interact` _output))))

(event `Key|P`
  (params (Key :type "Key Structure"))
  (bind _returnvalue (`GameplayStatics.GetPlayerController` 0))
  (bind _returnvalue_2 (`GameplayStatics.GetPlayerController` 0))
  (bind _menu (`self.Menu`))
  ;[0.5528 1 0.4499] Opens up the pause screen when the player presses 'P'
  (:`Pressed`
    (bind _returnvalue_3 (`|CreateWidget` "/Game/UI/PauseMenu.PauseMenu_C" _returnvalue _returnvalue))
    (set `self.Menu` _returnvalue_3)
    (set `PlayerController.bShowMouseCursor` true _returnvalue_2)
    (`WidgetBlueprintLibrary.SetInputMode_UIOnlyEx` _returnvalue_2 _menu)
    (`UserWidget.AddToViewport` _menu 0)
    (`GameplayStatics.SetGamePaused` true)))

(event `InputAxis|MoveForward`
  (params (AxisValue :type "Float (single-precision)"))
  ;[0.5528 1 0.4499] Handles the player movement controls
  (`self.AddMovementInput` (`KismetMathLibrary.GetForwardVector` (`KismetMathLibrary.MakeRotator` 0.0 0.0 (.yaw (`self.GetControlRotation`)))) AxisValue))

(event `InputAxis|MoveRight`
  (params (AxisValue :type "Float (single-precision)"))
  ;[0.5528 1 0.4499] Handles the player movement controls
  (`self.AddMovementInput` (`KismetMathLibrary.GetRightVector` (`KismetMathLibrary.MakeRotator` 0.0 0.0 (.yaw (`self.GetControlRotation`)))) AxisValue))

(event `InputAxis|LookUp`
  (params (AxisValue :type "Float (single-precision)"))
  ;[0.5528 1 0.4499] Handles the player movement controls
  (`self.AddControllerPitchInput` AxisValue))

(event `InputAxis|Turn`
  (params (AxisValue :type "Float (single-precision)"))
  ;[0.5528 1 0.4499] Handles the player movement controls
  (`self.AddControllerYawInput` AxisValue))

(event `InputAction|Jump`
  (params (Key :type "Key Structure"))
  ;[0.5528 1 0.4499] Handles the player movement controls
  (:`Pressed`
    (`self.Jump`))
  (:`Released`
    (`self.StopJumping`)))

(event `InputAction|Sprint`
  (params (Key :type "Key Structure"))
  (bind _charactermovement (`self.CharacterMovement`))
  ;[0.5528 1 0.4499] Handles the player movement controls
  (:`Pressed`
    (set `CharacterMovementComponent.MaxWalkSpeed` 1000.0 _charactermovement))
  (:`Released`
    (set `CharacterMovementComponent.MaxWalkSpeed` 600.0 _charactermovement)))

(event `self.ReceiveBeginPlay`
  (bind _returnvalue (`|CreateWidget` "/Game/UI/HealthBar.HealthBar_C"))
  (bind _output_get (set `self.Healthbarrref` _returnvalue))
  (`UserWidget.AddToViewport` _output_get 0))

(event `self.ReceiveAnyDamage`
  (params (Damage :type "Float (single-precision)") (DamageType :type "DamageType Object Reference") (InstigatedBy :type "Controller Object Reference") (DamageCauser :type "Actor Object Reference"))
  (set `self.Health` (`KismetMathLibrary.FClamp` (- (`self.Health`) Damage) 0.0 (`self.MaxHealth`)))
  (`/Game/UI/HealthBar.UpdateHealthBar` (`self.Healthbarrref`)))

(event `Key|One`
  (params (Key :type "Key Structure"))
  (:`Pressed`
    (`GameplayStatics.ApplyDamage` self 10.0)))

(fn `UserConstructionScript`)